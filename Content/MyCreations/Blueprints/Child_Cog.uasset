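; Child cog Blueprint: an interactable valve-like ring that fills or drains a gauge while the player turns it.
; Overlapping its collision flags the cog as interactable on FirstPersonCharacter and makes it turnable.
; Tick repeatedly binds TurnWheel and Stop to the character's dispatchers.
; TurnWheel rolls the ring while left mouse is held, changing the clamped gauge by frame time; Stop reverses direction, as does reaching maximum.
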(event OnComponentBeginOverlap(CollisionCheckPlayer)
  (params (OverlappedComponent :type Primitive%20Component%20Object%20Reference) (OtherActor :type Actor%20Object%20Reference) (OtherComp :type Primitive%20Component%20Object%20Reference) (OtherBodyIndex :type Integer) (bFromSweep :type Boolean) (SweepResult :type Hit%20Result%20Structure%20%28by%20ref%29))
  (bind _asfirst_person_character (Utilities|Casting|CastToFirstPersonCharacter OtherActor))
  (bind _output_get (Variables|Default|SetCharacter%20Ref _asfirst_person_character))
  (Variables|/Game/FirstPersonBP/Blueprints/FirstPersonCharacter.FirstPersonCharacter_C|SetCogIsInteractable _output_get true)
  (Variables|Default|SetTurnable true)
  (Variables|/Game/FirstPersonBP/Blueprints/FirstPersonCharacter.FirstPersonCharacter_C|SetIsCog _asfirst_person_character true)
  (Variables|Default|SetCanInteract? true))

(event OnComponentEndOverlap(CollisionCheckPlayer)
  (params (OverlappedComponent :type Primitive%20Component%20Object%20Reference) (OtherActor :type Actor%20Object%20Reference) (OtherComp :type Primitive%20Component%20Object%20Reference) (OtherBodyIndex :type Integer))
  (bind _asfirst_person_character (Utilities|Casting|CastToFirstPersonCharacter OtherActor))
  (Variables|/Game/FirstPersonBP/Blueprints/FirstPersonCharacter.FirstPersonCharacter_C|SetCogIsInteractable _asfirst_person_character false)
  (Variables|Default|SetTurnable false)
  (Variables|/Game/FirstPersonBP/Blueprints/FirstPersonCharacter.FirstPersonCharacter_C|SetIsCog _asfirst_person_character false)
  (Variables|Default|SetCanInteract? false))

(event Custom|TurnWheel
  (bind _pipe_detailring (Variables|Default|GetPipe_DetailRing))
  (bind _pipe_detailring_2 (Variables|Default|GetPipe_DetailRing))
  (bind _returnvalue (Transformation|GetWorldRotation _pipe_detailring_2))
  (bind _returnvalue_2 (Transformation|GetWorldRotation _pipe_detailring))
  (if (Game|Player|IsInputKeyDown (Game|GetPlayerController 0) "LeftMouseButton")
    (if (Variables|Default|GetFlipCondition)
      ;[1 1 1] Turn Cog right and add to gaugeAmount
      (Variables|Default|SetCurrentGaugeAmount (Math|Float|Clamp(Float) (+ (Variables|Default|GetCurrentGaugeAmount) (* (* (Variables|Default|GetGaugeFillAmount) (Utilities|Time|GetWorldDeltaSeconds)) 5.0)) 0.0 (Variables|Default|GetGaugeMax)))
      (Transformation|SetWorldRotation _pipe_detailring_2 (Math|Rotator|MakeRotator (+ (.roll _returnvalue) (Variables|Default|GetRotationspeed)) (.pitch _returnvalue) (.yaw _returnvalue)) false false)
      (if (>= (Variables|Default|GetCurrentGaugeAmount) (Variables|Default|GetGaugeMax))
        (Variables|Default|SetTurnable false)
        (Variables|Default|SetFlipCondition false))
      (else
        ;[1 1 1] Turn Cog left and subtract from gaugeAmount
        (Variables|Default|SetCurrentGaugeAmount (Math|Float|Clamp(Float) (- (Variables|Default|GetCurrentGaugeAmount) (* (* (Variables|Default|GetGaugeFillAmount) (Utilities|Time|GetWorldDeltaSeconds)) 5.0)) 0.0 (Variables|Default|GetGaugeMax)))
        (Transformation|SetWorldRotation _pipe_detailring (Math|Rotator|MakeRotator (- (.roll _returnvalue_2) (Variables|Default|GetRotationspeed)) (.pitch _returnvalue_2) (.yaw _returnvalue_2)) false false)
        (if (Math|Boolean|NotEqual(Boolean) (Variables|Default|GetTurnable) true)
          (Variables|Default|SetFlipCondition true))))))

(event Custom|Stop
  (if (Variables|Default|GetFlipCondition)
    (Variables|Default|SetFlipCondition false)
    (else
      (Variables|Default|SetFlipCondition true)))
  (Variables|Default|SetIsInteracting false))

(event EventTick
  (params (DeltaSeconds :type Float%20%28single-precision%29))
  (Utilities|FlowControl|Sequence
    (:then_0
      (if (Variables|Default|GetTurnable)
        (EventDispatchers|BindEventtoTurnCog (Variables|Default|GetCharacter%20Ref) (delegate Custom|TurnWheel))
        (Variables|Default|SetIsInteracting true)))
    (:then_1
      (bind _asfirst_person_character (Utilities|Casting|CastToFirstPersonCharacter (Game|GetPlayerCharacter 0)))
      (EventDispatchers|BindEventtoStopTurning _asfirst_person_character (delegate Custom|Stop)))))

(fn ConstructionScript
  (|CallParentFunction))