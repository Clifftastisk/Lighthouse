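; Interactable oil barrel that refills the first-person character's torch oil.
; On overlap it casts to FirstPersonCharacter and binds its replenish event to that character's fill-oil event.
; When that event fires while CanInteract and IsInteracting are true, it sets TorchOil to a full fixed amount and unbinds itself.
; The graph has no end-overlap handling, so the binding persists until a successful refill.
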(event Custom|Replenish%20oil
  (if (and (Variables|Default|GetCanInteract?) (Variables|Default|GetIsInteracting))
    (Variables|/Game/FirstPersonBP/Blueprints/FirstPersonCharacter.FirstPersonCharacter_C|SetTorchOil (stale Collision|EventActorBeginOverlap _asfirst_person_character) 1e+02)
    (EventDispatchers|UnbindEventfromFillOil (stale Collision|EventActorBeginOverlap _asfirst_person_character) (delegate Custom|Replenish%20oil))))

(event Collision|EventActorBeginOverlap
  (params (OtherActor :type Actor%20Object%20Reference))
  (bind _asfirst_person_character (Utilities|Casting|CastToFirstPersonCharacter OtherActor))
  (EventDispatchers|BindEventtoFillOil _asfirst_person_character (delegate Custom|Replenish%20oil)))

(fn ConstructionScript
  (|CallParentFunction))