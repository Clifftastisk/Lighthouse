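; Interactable world torch that lights from the player's lit torch and acts as a heat source.
; Each tick, while interaction is allowed and active and the player's TorchLit is set, it shows its particle effect.
; Overlap events track whether the player is in heat range, and under those same conditions it feeds warmth to the FirstPersonCharacter every frame.
; Nothing here hides the flame again.
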(event EventBeginPlay
  (|CallParentFunction)
  (Input|EnableInput (Game|GetPlayerController 0)))

(event EventTick
  (params (DeltaSeconds :type Float%20%28single-precision%29))
  (|CallParentFunction DeltaSeconds)
  (bind _asfirst_person_character (Utilities|Casting|CastToFirstPersonCharacter (Game|GetPlayerCharacter 0)))
  (if (Math|Boolean|ANDBoolean (Variables|Default|GetCanInteract?) (Variables|Default|GetIsInteracting) (Variables|/Game/FirstPersonBP/Blueprints/FirstPersonCharacter.FirstPersonCharacter_C|GetTorchLit _asfirst_person_character))
    (Rendering|SetVisibility (Variables|Default|GetParticleSystem) true true)
    (if (Variables|Default|GetInHeatRange)
      (Default|HeatSourceWarmth _asfirst_person_character 2.0))))

(event Collision|EventActorBeginOverlap
  (params (OtherActor :type Actor%20Object%20Reference))
  (Utilities|Casting|CastToFirstPersonCharacter OtherActor)
  (Variables|Default|SetInHeatRange true))

(event Collision|EventActorEndOverlap
  (params (OtherActor :type Actor%20Object%20Reference))
  (Utilities|Casting|CastToFirstPersonCharacter OtherActor)
  (Variables|Default|SetInHeatRange false))

(fn ConstructionScript
  (|CallParentFunction))