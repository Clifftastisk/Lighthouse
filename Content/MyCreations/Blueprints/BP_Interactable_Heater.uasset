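; Interactable stove heater that burns fuel to light up and warm the first-person player while they overlap it.
; BeginPlay seeds the CogRef gauge and stove widget from its fuel variables and binds the player's item effect to add fuel.
; During interaction, Tick derives consumption rate from the cog gauge and updates the widget.
; While fuel remains, Tick drains it by that rate and scales light intensity with the gauge.
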(event Custom|ItemEffect
  ;[1 1 1] Setting up all variables in the stove based off of the widget ones.Then sends into widget
  (if (Variables|Default|GetTakesFuel?)
    (Variables|Default|SetCurrentFuel (+ (Variables|Default|GetCurrentFuel) (Variables|Default|GetFuelToAdd)))))

(event EventBeginPlay
  (bind _cogref (Variables|Default|GetCogRef))
  ;[1 1 1] Setting up all variables in the stove based off of the widget ones.Then sends into widget
  (|CallParentFunction)
  (Input|EnableInput (Game|GetPlayerController 0))
  (Components|Activation|SetActive (Variables|Transformation|GetRootComponent) false false)
  (bind _output_get (Variables|Default|SetWidgetRef (UserInterface|GetUserWidgetObject (Variables|Default|GetWidget))))
  (bind _asstove_widget (Utilities|Casting|CastToStoveWidget _output_get))
  (bind _output_get_2 (Variables|/Game/MyCreations/Blueprints/Child_Cog.Child_Cog_C|SetGaugeMax _cogref (Variables|Default|GetFuelMaxStove)))
  (bind _output_get_3 (Variables|/Game/MyCreations/Blueprints/Child_Cog.Child_Cog_C|SetCurrentGaugeAmount _cogref (Variables|Default|GetCurrentFuel)))
  (Default|UpdateFuel _asstove_widget 0.0 _output_get_3 _output_get_2)
  (bind _asfirst_person_character (Utilities|Casting|CastToFirstPersonCharacter (Game|GetPlayerCharacter 0)))
  (EventDispatchers|BindEventtoItemEffect _asfirst_person_character (delegate Custom|ItemEffect)))

(event EventTick
  (params (DeltaSeconds :type Float%20%28single-precision%29))
  (bind _cogref (Variables|Default|GetCogRef))
  ;[1 1 1] Interaction logic - Send information to the widget
  (|CallParentFunction DeltaSeconds)
  (Utilities|FlowControl|Sequence
    (:then_0
      (if (Variables|Default|GetIsInteracting)
        (bind _asstove_widget (Utilities|Casting|CastToStoveWidget (Variables|Default|GetWidgetRef)))
        (Default|ModifyFuel _asstove_widget (Variables|Default|GetCurrentFuel) (Variables|Default|GetConsumptionRate))
        (bind _output_get (Variables|Default|SetConsumptionRate (* (+ (Variables|/Game/MyCreations/Blueprints/Child_Cog.Child_Cog_C|GetCurrentGaugeAmount _cogref) (Variables|/Game/MyCreations/Blueprints/Child_Cog.Child_Cog_C|GetGaugeFillAmount _cogref)) 3.0)))
        (Default|ModifyConsumption _asstove_widget _output_get)))
    (:then_1
      ;[1 1 1] Increases Fire light in the stove based off of the consumption rate
      (if (Variables|Default|GetIsThereFuel)
        (Rendering|Components|Light|SetIntensity (Variables|Default|GetPointLight) (* (Variables|/Game/MyCreations/Blueprints/Child_Cog.Child_Cog_C|GetCurrentGaugeAmount (Variables|Default|GetCogRef)) 2.0))
        (bind _asfirst_person_character (Utilities|Casting|CastToFirstPersonCharacter (Game|GetPlayerCharacter 0)))
        (if (Collision|IsOverlappingActor _asfirst_person_character :!class /Script/Engine.Actor)
          (Default|HeatSourceWarmth _asfirst_person_character (Variables|Default|GetTemperatureIncrease)))))
    (:then_2
      ;[1 1 1] If there is fuel, start decrease
      (if (Variables|Default|GetIsThereFuel)
        (Variables|Default|SetCurrentFuel (- (Variables|Default|GetCurrentFuel) (* (* (Variables|Default|GetConsumptionRate) (Utilities|Time|GetWorldDeltaSeconds)) 0.03)))))
    (:then_3
      (if (> (Variables|Default|GetCurrentFuel) 1.0)
        (Variables|Default|SetIsThereFuel true)
        (if (> (Variables|Default|GetCurrentFuel) 1e+02)
          (Variables|Default|SetCurrentFuel 99.0))
        (else
          (Variables|Default|SetIsThereFuel false))))))

(fn ConstructionScript
  (|CallParentFunction))