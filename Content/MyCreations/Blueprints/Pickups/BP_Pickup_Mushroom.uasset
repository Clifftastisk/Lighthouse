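; Mushroom pickup that goes into the player's inventory and, when used, changes health and hunger and makes the player Sick for a few seconds.
; BeginPlay builds its prompt widget and item struct, then binds pickup to the first-person character.
; Overlap shows or removes the prompt, gated by CanInteract.
; Pickup adds the item, refreshes the HUD inventory, and hides the actor without destroying it.
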(event OnComponentBeginOverlap(OverlapCheck)
  (params (OverlappedComponent :type Primitive%20Component%20Object%20Reference) (OtherActor :type Actor%20Object%20Reference) (OtherComp :type Primitive%20Component%20Object%20Reference) (OtherBodyIndex :type Integer) (bFromSweep :type Boolean) (SweepResult :type Hit%20Result%20Structure%20%28by%20ref%29))
  ;[1 1 1] Overlap Trigger for the PickupWidget
  (Utilities|Casting|CastToFirstPersonCharacter OtherActor)
  (if (Variables|Default|GetCanInteract?)
    (UserInterface|Viewport|AddtoViewport (Variables|Default|GetPickupTextReference) 0)
    (if (Variables|Default|GetIsInteracting)
      _)))

(event OnComponentEndOverlap(OverlapCheck)
  (params (OverlappedComponent :type Primitive%20Component%20Object%20Reference) (OtherActor :type Actor%20Object%20Reference) (OtherComp :type Primitive%20Component%20Object%20Reference) (OtherBodyIndex :type Integer))
  ;[1 1 1] Overlap Trigger for the PickupWidget
  (Utilities|Casting|CastToFirstPersonCharacter OtherActor)
  (Widget|RemovefromParent (Variables|Default|GetPickupTextReference))
  (Variables|Default|SetCanInteract? false))

(event Custom|PickupItem_Event_0
  (bind _characterreference (Variables|Default|GetCharacterReference))
  (bind _gamehudreference (Variables|/Game/FirstPersonBP/Blueprints/FirstPersonCharacter.FirstPersonCharacter_C|GetGameHudReference _characterreference))
  ;[1 1 1] Pickup and add items to inventory then refresh it
  (if (and (Variables|Default|GetCanInteract?) (Collision|GetActorEnableCollision))
    (Utilities|Array|Add (Variables|/Game/MyCreations/Widgets/GameHud.GameHud_C|GetInventoryWidget _gamehudreference) (Variables|Default|GetItemInfo))
    (Widget|RemovefromParent (Variables|Default|GetPickupTextReference))
    (Rendering|SetActorHiddenInGame true)
    (Collision|SetActorEnableCollision false)
    (Default|RefreshInventory _gamehudreference)))

(event EventBeginPlay
  (bind _iteminfo (Variables|Default|GetItemInfo))
  (bind (_item _itemimage _pickuptext) (Utilities|Struct|BreakInventoryStruct _iteminfo))
  ;[1 1 1] Event beginplay - setting all the variables for the instance of pickup
  (bind _returnvalue (UserInterface|CreateWidget "/Game/MyCreations/Widgets/PickupWidget.PickupWidget_C"))
  (Variables|Default|SetPickupTextReference _returnvalue)
  (Utilities|Struct|SetmembersinInventoryStruct _iteminfo self)
  (Variables|/Game/MyCreations/Widgets/PickupWidget.PickupWidget_C|SetPickupActor (Variables|Default|GetPickupTextReference) _item)
  (Variables|/Game/MyCreations/Widgets/PickupWidget.PickupWidget_C|SetPickupText (Variables|Default|GetPickupTextReference) _pickuptext)
  (bind _asfirst_person_character (Utilities|Casting|CastToFirstPersonCharacter (Game|GetPlayerCharacter 0)))
  (bind _output_get (Variables|Default|SetCharacterReference _asfirst_person_character))
  (EventDispatchers|AssignPickupItem _output_get (delegate Custom|PickupItem_Event_0)))

(event EventUseAction
  (bind _characterreference (Variables|Default|GetCharacterReference))
  ;[1 1 1] Use Action
  (Variables|/Game/FirstPersonBP/Blueprints/FirstPersonCharacter.FirstPersonCharacter_C|SetHealth%20Amount _characterreference (+ (Variables|/Game/FirstPersonBP/Blueprints/FirstPersonCharacter.FirstPersonCharacter_C|GetHealth%20Amount _characterreference) (Variables|Default|GetAddHealth)))
  (Variables|/Game/FirstPersonBP/Blueprints/FirstPersonCharacter.FirstPersonCharacter_C|SetHungerAmount _characterreference (+ (Variables|/Game/FirstPersonBP/Blueprints/FirstPersonCharacter.FirstPersonCharacter_C|GetHungerAmount _characterreference) (Variables|Default|GetRemoveHunger)))
  (bind _asfirst_person_character (Utilities|Casting|CastToFirstPersonCharacter (Game|GetPlayerCharacter 0)))
  (Variables|/Game/FirstPersonBP/Blueprints/FirstPersonCharacter.FirstPersonCharacter_C|SetSick _asfirst_person_character true)
  (Utilities|FlowControl|Delay 6.0)
  (Variables|/Game/FirstPersonBP/Blueprints/FirstPersonCharacter.FirstPersonCharacter_C|SetSick _asfirst_person_character false))

(fn ConstructionScript
  (|CallParentFunction)
  (if (Variables|Default|GetIsCustomMesh)
    (Components|StaticMesh|SetStaticMesh (Variables|Default|GetMesh) (Variables|Default|GetStatic%20Mesh))))