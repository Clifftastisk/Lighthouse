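; BP_ZoneMaster is an environmental hazard zone that affects the first-person character while inside it.
; Overlap start caches the character and starts looping two-second timers for whichever heated, cold or nausea flags are set.
; Timer events raise or lower temperature and update the HUD, or mark the player sick with a debug print.
; Any overlap end clears the Inside flag gating these events, but the timers are never cleared.
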(event Custom|Nausiate
  (if (Variables|Default|GetInside)
    (Variables|/Game/FirstPersonBP/Blueprints/FirstPersonCharacter.FirstPersonCharacter_C|SetSick (stale Collision|EventActorBeginOverlap _asfirst_person_character) true)
    (Development|PrintString "Down with the sickness")))

(event Custom|Lower%20Temperature
  (if (Variables|Default|GetInside)
    (bind _output_get (Variables|/Game/FirstPersonBP/Blueprints/FirstPersonCharacter.FirstPersonCharacter_C|SetTemperature (stale Collision|EventActorBeginOverlap _asfirst_person_character) (- (Variables|/Game/FirstPersonBP/Blueprints/FirstPersonCharacter.FirstPersonCharacter_C|GetTemperature (stale Collision|EventActorBeginOverlap _asfirst_person_character)) 0.3)))
    (Default|ModifyTemp (Variables|/Game/FirstPersonBP/Blueprints/FirstPersonCharacter.FirstPersonCharacter_C|GetGameHudReference (stale Collision|EventActorBeginOverlap _asfirst_person_character)) _output_get)))

(event Custom|Raise%20Temperature
  (if (Variables|Default|GetInside)
    (bind _output_get (Variables|/Game/FirstPersonBP/Blueprints/FirstPersonCharacter.FirstPersonCharacter_C|SetTemperature (stale Collision|EventActorBeginOverlap _asfirst_person_character) (+ (Variables|/Game/FirstPersonBP/Blueprints/FirstPersonCharacter.FirstPersonCharacter_C|GetTemperature (stale Collision|EventActorBeginOverlap _asfirst_person_character)) 0.3)))
    (Default|ModifyTemp (Variables|/Game/FirstPersonBP/Blueprints/FirstPersonCharacter.FirstPersonCharacter_C|GetGameHudReference (stale Collision|EventActorBeginOverlap _asfirst_person_character)) _output_get)))

(event Collision|EventActorEndOverlap
  (params (OtherActor :type Actor%20Object%20Reference))
  (Variables|Default|SetInside false))

(event Collision|EventActorBeginOverlap
  (params (OtherActor :type Actor%20Object%20Reference))
  (bind _asfirst_person_character (Utilities|Casting|CastToFirstPersonCharacter OtherActor))
  (Variables|Default|SetInside true)
  (Utilities|FlowControl|Sequence
    (:then_0
      (if (Variables|Default|GetHeatedArea)
        (Utilities|Time|SetTimerbyEvent (delegate Custom|Raise%20Temperature) 2.0 (Variables|Default|GetInside))))
    (:then_1
      (if (Variables|Default|GetColdArea)
        (Utilities|Time|SetTimerbyEvent (delegate Custom|Lower%20Temperature) 2.0 (Variables|Default|GetInside))))
    (:then_2
      (if (Variables|Default|GetNauseaArea)
        (Utilities|Time|SetTimerbyEvent (delegate Custom|Nausiate) 2.0 (Variables|Default|GetInside))))))

(fn ConstructionScript)