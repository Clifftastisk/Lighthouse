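; Master Blueprint for a possessable pawn that the player's FirstPersonCharacter can take control of and later exit.
; Entering its Collision binds PossessThing to the character's Possess dispatcher, and leaving clears all bindings on that dispatcher.
; PossessThing stores the player character and possesses this pawn.
; Pressing E moves that character to ExitPosition, restores its saved OriginalRotation on controller and actor, then repossesses it.
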(event OnComponentBeginOverlap(Collision)
  (params (OverlappedComponent :type Primitive%20Component%20Object%20Reference) (OtherActor :type Actor%20Object%20Reference) (OtherComp :type Primitive%20Component%20Object%20Reference) (OtherBodyIndex :type Integer) (bFromSweep :type Boolean) (SweepResult :type Hit%20Result%20Structure%20%28by%20ref%29))
  ;[1 1 1] Possesion logic
  (bind _asfirst_person_character (Utilities|Casting|CastToFirstPersonCharacter OtherActor))
  (EventDispatchers|BindEventtoPossess _asfirst_person_character (delegate Custom|PossessThing)))

(event OnComponentEndOverlap(Collision)
  (params (OverlappedComponent :type Primitive%20Component%20Object%20Reference) (OtherActor :type Actor%20Object%20Reference) (OtherComp :type Primitive%20Component%20Object%20Reference) (OtherBodyIndex :type Integer))
  ;[1 1 1] Possesion logic
  (bind _asfirst_person_character (Utilities|Casting|CastToFirstPersonCharacter OtherActor))
  (EventDispatchers|UnbindallEventsfromPossess _asfirst_person_character))

(event Custom|PossessThing
  ;[1 1 1] Possesion logic
  (Variables|Default|SetCharacterRef (Game|GetPlayerCharacter 0))
  (Pawn|Possess (Game|GetPlayerController 0) self))

(event Input|KeyboardEvents|E
  (params (Key :type Key%20Structure :default "None"))
  (bind _characterref (Variables|Default|GetCharacterRef))
  (bind _characterref_2 (Variables|Default|GetCharacterRef))
  ;[1 1 1] Exit logic
  (:Pressed
    (Transformation|SetActorTransform _characterref_2 (Transformation|GetWorldTransform (Variables|Default|GetExitPosition)))
    (bind _asfirst_person_character (Utilities|Casting|CastToFirstPersonCharacter _characterref))
    (Pawn|SetControlRotation (Game|GetPlayerController 0) (Variables|/Game/FirstPersonBP/Blueprints/FirstPersonCharacter.FirstPersonCharacter_C|GetOriginalRotation _asfirst_person_character))
    (Transformation|SetActorRotation _characterref (Variables|/Game/FirstPersonBP/Blueprints/FirstPersonCharacter.FirstPersonCharacter_C|GetOriginalRotation _asfirst_person_character))
    (Pawn|Possess (Game|GetPlayerController 0) _characterref_2)))

(fn ConstructionScript)